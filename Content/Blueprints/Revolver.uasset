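; Revolver Blueprint that tracks a six-chamber cylinder (Barillet) with a loaded flag per chamber and rotates it to open or close.
; LoadBullet matches the given chamber component to its flag and sets it, without changing the material.
; Fire advances a wrapping index mapped to chambers out of numeric order, then returns whether that chamber was loaded, clearing it and applying the empty material if so.
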(fn ConstructionScript)

(fn LoadBullet
  (params (chambreToLoad :type Primitive%20Component%20Object%20Reference))
  (if (== chambreToLoad (Variables|Default|GetChambre%200))
    (Variables|Default|SetChamber%201%20loaded true)
    (elif (== chambreToLoad (Variables|Default|GetChambre%201))
      (Variables|Default|SetChamber%202%20loaded true)
      (elif (== chambreToLoad (Variables|Default|GetChambre%202))
        (Variables|Default|SetChamber%203%20loaded true)
        (elif (== chambreToLoad (Variables|Default|GetChambre%203))
          (Variables|Default|SetChamber%204%20loaded true)
          (elif (== chambreToLoad (Variables|Default|GetChambre%204))
            (Variables|Default|SetChamber%205%20loaded true)
            (elif (== chambreToLoad (Variables|Default|GetChambre%205))
              (Variables|Default|SetChamber%206%20loaded true))))))))

(fn OpenBarillet
  (Transformation|SetRelativeRotation (Variables|Default|Getbarillet) "90.000000, 0, 0" false false))

(fn CloseBarillet
  (Transformation|SetRelativeRotation (Variables|Default|Getbarillet) "0, 0, 0" false false))

(fn Fire
  (bind _output_get (Variables|Default|SetChamber%20to%20fire%20index (Math|Integer|%(Integer) (+ (Variables|Default|GetChamber%20to%20fire%20index) 1) 6)))
  (switch int _output_get
    (:Default
      (return false))
    (:0
      (if (Variables|Default|GetChamber%201%20loaded)
        (Variables|Default|SetChamber%201%20loaded false)
        (Rendering|Material|SetMaterial (Variables|Default|GetChambre%200) 0 "/Game/Graphics/Materials/Weapon/EmptyChamber.EmptyChamber")
        (return true)
        (else
          (return false))))
    (:1
      (if (Variables|Default|GetChamber%206%20loaded)
        (Variables|Default|SetChamber%206%20loaded false)
        (Rendering|Material|SetMaterial (Variables|Default|GetChambre%205) 0 "/Game/Graphics/Materials/Weapon/EmptyChamber.EmptyChamber")
        (return true)
        (else
          (return false))))
    (:2
      (if (Variables|Default|GetChamber%203%20loaded)
        (Variables|Default|SetChamber%203%20loaded false)
        (Rendering|Material|SetMaterial (Variables|Default|GetChambre%202) 0 "/Game/Graphics/Materials/Weapon/EmptyChamber.EmptyChamber")
        (return true)
        (else
          (return false))))
    (:3
      (if (Variables|Default|GetChamber%202%20loaded)
        (Variables|Default|SetChamber%202%20loaded false)
        (Rendering|Material|SetMaterial (Variables|Default|GetChambre%201) 0 "/Game/Graphics/Materials/Weapon/EmptyChamber.EmptyChamber")
        (return true)
        (else
          (return false))))
    (:4
      (if (Variables|Default|GetChamber%204%20loaded)
        (Variables|Default|SetChamber%204%20loaded false)
        (Rendering|Material|SetMaterial (Variables|Default|GetChambre%203) 0 "/Game/Graphics/Materials/Weapon/EmptyChamber.EmptyChamber")
        (return true)
        (else
          (return false))))
    (:5
      (if (Variables|Default|GetChamber%205%20loaded)
        (Variables|Default|SetChamber%205%20loaded false)
        (Rendering|Material|SetMaterial (Variables|Default|GetChambre%204) 0 "/Game/Graphics/Materials/Weapon/EmptyChamber.EmptyChamber")
        (return true)
        (else
          (return false))))))